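; Ice crystal hazard that explodes after taking lethal damage, dealing ice damage to nearby actors.
; Any damage disables collision, and only the first hit reduces health; if lethal, it spawns particles and starts a detonation timer.
; ExplodeCrystal damages actors overlapping the explosion volume and flags WasAttacked, so Tick destroys the crystal after a short delay.
; BeginPlay configures the ice effect damage, and DisableTrap removes the actor.
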(event `self.ReceiveBeginPlay`
  (bind _icetype (`/Game/Blueprints/Libraries/BP_Actor_FunctionLibrary.IceDamageType` self))
  (`/Game/Blueprints/Libraries/BP_Actor_FunctionLibrary.SetEffectDamage` _icetype (`self.EffectDamage`)))

(event `self.ReceiveAnyDamage`
  (params (Damage :type "Float (single-precision)") (DamageType :type "DamageType Object Reference") (InstigatedBy :type "Controller Object Reference") (DamageCauser :type "Actor Object Reference"))
  (`PrimitiveComponent.SetCollisionResponseToAllChannels` (`self.Cube`) "ECR_Ignore")
  (`PrimitiveComponent.SetCollisionResponseToAllChannels` (`self.Box`) "ECR_Ignore")
  (if (`self.isAlive`)
    (bind _output_get (set `self.health` (- (`self.health`) Damage)))
    (set `self.isAlive` false)
    (if (and (<= _output_get 0.0) (not (`self.isAlive`)))
      (`GameplayStatics.SpawnEmitterAttached` "/Game/VFX/CrystalTrap/PS_CrystalPart1.PS_CrystalPart1" (`self.Cube`) "None" (0.0 0.0 0.0) (struct) (0.5 0.5 0.5))
      (`KismetSystemLibrary.K2_SetTimer` self "ExplodeCrystal" (`self.detonationTime`)))))

(event `self.DisableTrap`
  (set `self.Enabled` false)
  (`self.K2_DestroyActor`))

(event `self.ReceiveTick`
  (params (DeltaSeconds :type "Float (single-precision)"))
  (if (`self.wasAttacked`)
    (`KismetSystemLibrary.Delay` 0.5)
    (`self.K2_DestroyActor`)))

(fn `ExplodeCrystal`
  (if (`self.Enabled`)
    (`PrimitiveComponent.SetCollisionResponseToAllChannels` (`self.Cube`) "ECR_Ignore")
    (`PrimitiveComponent.SetCollisionResponseToAllChannels` (`self.Box`) "ECR_Ignore")
    (bind _returnvalue (`GameplayStatics.SpawnEmitterAttached` "/Game/VFX/CrystalTrap/PS_CrystalPart2.PS_CrystalPart2" (`self.Cube`) "None" (0.0 0.0 0.0) (struct) (0.2 0.2 0.2)))
    (set `self.explosionVFX` _returnvalue)
    (for _array_element (`PrimitiveComponent.GetOverlappingActors` (`self.ExplosionCollision`) "/Script/Engine.Actor")
      (`GameplayStatics.ApplyDamage` _array_element (`self.damage`) null self "/Game/Blueprints/DamageType_Ice.DamageType_Ice_C"))
    (set `self.wasAttacked` true)))

(fn `UserConstructionScript`
  (`parent.UserConstructionScript`))
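; Snowball launcher hazard that fires BP_SnowballHazard projectiles carrying ice damage, set up at BeginPlay.
; LaunchProjectile, while enabled, plays the launch animation, then after a short delay spawns the snowball at the child actor's location and rotation.
; A DoOnce allows one shot until Reload waits ReloadTime, marks it loaded and resets the gate.
; DisableTrap blocks further launches, and the Launch function is an empty stub.
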(event `self.ReceiveBeginPlay`
  (`parent.ReceiveBeginPlay`)
  (bind _icetype (`/Game/Blueprints/Libraries/BP_Actor_FunctionLibrary.IceDamageType` self))
  (bind _output_get (set `self.damageType` _icetype))
  (`/Game/Blueprints/Libraries/BP_Actor_FunctionLibrary.SetEffectDamage` _output_get (`self.effectDamage`)))

(event `LaunchProjectile`
  (bind _childactor (`self.ChildActor`))
  (if (`self.Enabled`)
    (`/Engine/EditorBlueprintResources/StandardMacros.DoOnce` false :!label _label
      (:`Completed`
        (`SkeletalMeshComponent.PlayAnimation` (`self.SkeletalMesh`) "/Game/Animations/Environment/Hazards/AM_Hazard_Snow_Trap_Launch_Montage.AM_Hazard_Snow_Trap_Launch_Montage" false)
        (`KismetSystemLibrary.Delay` 0.6)
        (`|SpawnActorFromClass` "/Game/Blueprints/Actors/Hazards/Ice_Hazards/BP_SnowballHazard.BP_SnowballHazard_C" (`KismetMathLibrary.MakeTransform` (`SceneComponent.K2_GetComponentLocation` _childactor) (`SceneComponent.K2_GetComponentRotation` _childactor)) "Undefined" "OverrideRootScale" null 4.0 (`self.damageType`) null null)
        (set `self.isLoaded` false)))))

(event `Reload`
  (`KismetSystemLibrary.Delay` (`self.reloadTime`))
  (set `self.isLoaded` true)
  (goto _label :!via `Reset`))

(event `self.DisableTrap`
  (set `self.Enabled` false))

(fn `Launch`)

(fn `UserConstructionScript`
  (`parent.UserConstructionScript`))
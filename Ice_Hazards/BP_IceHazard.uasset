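; Ice hazard Blueprint that periodically damages and applies an ice status effect to actors inside its box volume.
; On BeginPlay it creates an ice damage type, configures it with its damage stats and starts a looping SlowActor timer.
; Each tick of that timer queries the box's overlapping actors, applying status effects with stack-ignoring enabled plus direct damage to each, rather than reacting to overlap events.
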(event `self.ReceiveBeginPlay`
  (set `self.ignoreStack` true)
  (bind _icetype (`/Game/Blueprints/Libraries/BP_Actor_FunctionLibrary.IceDamageType` self))
  (bind _output_get (set `self.DamageTypeRef` _icetype))
  (`/Game/Blueprints/Libraries/BP_Actor_FunctionLibrary.SetEffectDamage` _output_get (`self.DamageNumbers`))
  (`KismetSystemLibrary.K2_SetTimer` self "SlowActor" (`self.damageOverTime`) true))

(fn `SlowActor`
  (for _array_element (`PrimitiveComponent.GetOverlappingActors` (`self.Box`) "/Script/Engine.Actor")
    (if true
      _
      (else
        _))
    (`/Game/Blueprints/Libraries/BP_Actor_FunctionLibrary.ApplyStatusEffects` _array_element (`self.DamageTypeRef`) self (`self.ignoreStack`))
    (`GameplayStatics.ApplyDamage` _array_element (`self.Damage`) null self)))

(fn `UserConstructionScript`
  (`parent.UserConstructionScript`))
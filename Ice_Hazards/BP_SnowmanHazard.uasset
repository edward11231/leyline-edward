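; Snowman ice hazard trap that attacks and damages actors in front of it.
; A Box overlap, while the trap is enabled, spawns a warning-style arch effect, waits a delay, then runs VisionCheck on the actors still inside.
; VisionCheck plays the attack animation and VFX per actor, but damages only those within VisionAngle of its forward vector, using a dot-product cone test.
; DisableTrap switches it off; the ice damage-type setup is unconnected.
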(event `self.ReceiveBeginPlay`
  (`parent.ReceiveBeginPlay`))

(event `Attack`
  (bind (_damageeffect_seconds _damageeffect_damage) (break `/Game/Blueprints/Attack/Struct_StatusEffectDamage` (`self.damageEffect`)))
  (`GameplayStatics.ApplyDamage` (`self.overlappedActor`) _damageeffect_damage))

(event `SpawnVFX`
  (`GameplayStatics.SpawnEmitterAttached` "/Game/VFX/Slimefolk/Snowman/PS_SnowmanAttack.PS_SnowmanAttack" (`self.Arrow`) "None" (0.0 0.0 0.0) (struct) (5.0 5.0 5.0)))

(event `self.Box.OnComponentBeginOverlap`
  (params (OverlappedComponent :type "PrimitiveComponent Object Reference") (OtherActor :type "Actor Object Reference") (OtherComp :type "PrimitiveComponent Object Reference") (OtherBodyIndex :type Integer) (bFromSweep :type Boolean) (SweepResult :type "HitResult Structure (by ref)"))
  (if (`self.Enabled`)
    (`GameplayStatics.SpawnEmitterAttached` "/Game/VFX/Slimefolk/Snowman/PS_SnowmanArch.PS_SnowmanArch" (`self.Arrow`) "None" (0.0 0.0 0.0) (struct) (7.0 7.0 7.0))
    (`KismetSystemLibrary.Delay` (`self.delayUntilAttack`))
    (`self.VisionCheck`)))

(event `self.DisableTrap`
  (set `self.Enabled` false))

(fn `UserConstructionScript`
  (`parent.UserConstructionScript`))

(fn `VisionCheck`
  (if (`self.Enabled`)
    (for _array_element (`PrimitiveComponent.GetOverlappingActors` (`self.Box`) "/Script/Engine.Actor")
      (bind _output_get (set `self.overlappedActor` _array_element))
      (`SkeletalMeshComponent.PlayAnimation` (`self.SkeletalMesh`) "/Game/Animations/Environment/Hazards/A_Hazard_Snowman_Trap_01A_Attack.A_Hazard_Snowman_Trap_01A_Attack" false)
      (`self.SpawnVFX`)
      (if (< (`KismetMathLibrary.DegAcos` (`KismetMathLibrary.Dot_VectorVector` (`self.GetActorForwardVector`) (`KismetMathLibrary.Normal` (- (`self.K2_GetActorLocation` _output_get) (`self.K2_GetActorLocation`))))) (`self.visionAngle`))
        (`self.Attack`)))))
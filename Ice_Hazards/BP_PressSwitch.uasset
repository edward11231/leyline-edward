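; Pressure switch for ice hazards that fires linked traps while an actor stands in its Box.
; Every Tick, if the first trap in TriggeredTrap is loaded, overlapping actors trigger LaunchProjectile, with the trap loop breaking after one call.
; Otherwise, Tick calls Reload on every linked trap.
; Overlap begin and end drive a timeline that lowers and raises the Cube, lerping from its start location toward an offset below its current position.
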(event `self.ReceiveBeginPlay`
  (set `self.startLocation` (`SceneComponent.K2_GetComponentLocation` (`self.Cube`))))

(event `self.ReceiveTick`
  (params (DeltaSeconds :type "Float (single-precision)"))
  (bind _triggeredtrap (`self.triggeredTrap`))
  (if (`/Game/Blueprints/Actors/Hazards/Ice_Hazards/BP_SnowballLauncher.isLoaded` (`|GetArrayItem` _triggeredtrap))
    (for _array_element (`PrimitiveComponent.GetOverlappingActors` (`self.Box`) "/Script/Engine.Actor") :!label _label
      (if (not (== _array_element self))
        (`/Engine/EditorBlueprintResources/StandardMacros.IsValid` _array_element
          (:`Is Valid`
            (for _array_element_2 (`self.triggeredTrap`)
              (`/Game/Blueprints/Actors/Hazards/Ice_Hazards/BP_SnowballLauncher.LaunchProjectile` _array_element_2)
              (goto _label :!via `Break`))))))
    (else
      (for _array_element_3 _triggeredtrap
        (`/Game/Blueprints/Actors/Hazards/Ice_Hazards/BP_SnowballLauncher.Reload` _array_element_3)))))

(event `self.Box.OnComponentBeginOverlap`
  (params (OverlappedComponent :type "PrimitiveComponent Object Reference") (OtherActor :type "Actor Object Reference") (OtherComp :type "PrimitiveComponent Object Reference") (OtherBodyIndex :type Integer) (bFromSweep :type Boolean) (SweepResult :type "HitResult Structure (by ref)"))
  (bind (_returnvalue_x _returnvalue_y _returnvalue_z) (`KismetMathLibrary.BreakVector` (`SceneComponent.K2_GetComponentLocation` (`self.Cube`))))
  (bind (_direction _alpha) (`Timeline|SwitchMovement` :!via `PlayFromStart` :!label _label_2)
    (:`Update`
      (`SceneComponent.K2_SetWorldLocation` (`self.Cube`) (`KismetMathLibrary.VLerp` (`self.startLocation`) (`KismetMathLibrary.MakeVector` _returnvalue_x _returnvalue_y (- _returnvalue_z (`self.switchPressLocation`))) _alpha) false false))))

(event `self.Box.OnComponentEndOverlap`
  (params (OverlappedComponent :type "PrimitiveComponent Object Reference") (OtherActor :type "Actor Object Reference") (OtherComp :type "PrimitiveComponent Object Reference") (OtherBodyIndex :type Integer))
  (goto _label_2 :!via `ReverseFromEnd`))

(fn `UserConstructionScript`)
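; Galawick candle fire hazard that detonates on a timer from BeginPlay, or earlier when the main character enters its sphere.
; Detonate runs only once, attaching a candle particle effect to the box and starting a delay before Explode.
; Explode applies damage to every actor overlapping the sphere, then destroys the hazard.
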(event `self.ReceiveBeginPlay`
  (`parent.ReceiveBeginPlay`)
  (`KismetSystemLibrary.K2_SetTimer` self "Detonate" (`self.detonationTime`)))

(event `self.Sphere.OnComponentBeginOverlap`
  (params (OverlappedComponent :type "PrimitiveComponent Object Reference") (OtherActor :type "Actor Object Reference") (OtherComp :type "PrimitiveComponent Object Reference") (OtherBodyIndex :type Integer) (bFromSweep :type Boolean) (SweepResult :type "HitResult Structure (by ref)"))
  (cast `/Game/Blueprints/Character/Elizabeth/BP_MainCharacter` OtherActor)
  (`self.Detonate`))

(fn `Detonate`
  (if (not (`self.detonateCalled`))
    (`KismetSystemLibrary.PrintString` "detonating...")
    (set `self.detonateCalled` true)
    ;[1 1 1] Play color changing animation
    (`GameplayStatics.SpawnEmitterAttached` "/Game/VFX/BossEnemy/PS_CameoCandle.PS_CameoCandle" (`self.Box`) "None" (0.0 0.0 -50.0) (struct) (1.5 1.5 1.5))
    (`KismetSystemLibrary.K2_SetTimer` self "Explode" (`self.detonationDelay`))))

(fn `Explode`
  (`KismetSystemLibrary.PrintString` "EXPLODE")
  (for _array_element (`PrimitiveComponent.GetOverlappingActors` (`self.Sphere`) "/Script/Engine.Actor")
    (`GameplayStatics.ApplyDamage` _array_element (`self.damage`)))
  (`self.K2_DestroyActor`))

(fn `UserConstructionScript`
  (`parent.UserConstructionScript`))
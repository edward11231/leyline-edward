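; Fire-hazard tree that topples when damaged and can hurt what it lands on.
; Only the first hit counts, felling it if health reaches zero.
; An arrow yaws relative to the damage causer, then a timeline rolls a child arrow carrying the trunk.
; On landing it passes the damage to capsule overlaps, destroys the trunk after a delay and credits an achievement if the player caused it.
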(event `self.ReceiveBeginPlay`
  (bind _asbp_game_instance (cast `/Game/Blueprints/BP_GameInstance` (`GameplayStatics.GetGameInstance`)))
  (set `self.InstanceRef` _asbp_game_instance))

(event `self.ReceiveAnyDamage`
  (params (Damage :type "Float (single-precision)") (DamageType :type "DamageType Object Reference") (InstigatedBy :type "Controller Object Reference") (DamageCauser :type "Actor Object Reference"))
  (bind _arrow (`self.Arrow`))
  (bind _trunk (`self.Trunk`))
  (bind _arrow1 (`self.Arrow1`))
  (bind _trunk_2 (`self.Trunk`))
  (bind (_returnvalue_roll _returnvalue_pitch _returnvalue_yaw) (`KismetMathLibrary.BreakRotator` (`KismetMathLibrary.FindLookAtRotation` (`SceneComponent.K2_GetComponentLocation` (`self.Arrow`)) (`self.K2_GetActorLocation` DamageCauser))))
  (set `self.Causer` DamageCauser)
  (if (`self.IsAlive`)
    (bind _output_get (set `self.Health` (- (`self.Health`) Damage)))
    (set `self.IsAlive` false)
    (if (and (<= _output_get 0.0) (not (`self.IsAlive`)))
      (`/Engine/EditorBlueprintResources/StandardMacros.IsValid` _arrow
        (:`Is Valid`
          (`SceneComponent.K2_SetWorldRotation` _arrow (`KismetMathLibrary.MakeRotator` 0.0 0.0 (+ _returnvalue_yaw 90.0)) false false)
          (`/Engine/EditorBlueprintResources/StandardMacros.IsValid` _arrow1
            (:`Is Valid`
              (`/Engine/EditorBlueprintResources/StandardMacros.IsValid` _trunk
                (:`Is Valid`
                  (`SceneComponent.K2_AttachToComponent` _trunk _arrow1 "None" "KeepWorld" "KeepWorld" "KeepRelative" false)
                  (`PrimitiveComponent.SetCollisionEnabled` _trunk "NoCollision")
                  (bind (_direction _fallpercent) (`Timeline|Fall over`)
                    (:`Update`
                      (`SceneComponent.K2_SetRelativeRotation` (`self.Arrow1`) (`KismetMathLibrary.MakeRotator` (* _fallpercent 110.0)) false false))
                    (:`Finished`
                      (for _array_element (`PrimitiveComponent.GetOverlappingActors` (`self.Capsule`) null)
                        (`GameplayStatics.ApplyDamage` _array_element (`self.Damage`) null self))
                      (`KismetSystemLibrary.Delay` 3.0)
                      (`/Engine/EditorBlueprintResources/StandardMacros.IsValid` _trunk_2
                        (:`Is Valid`
                          (`ActorComponent.K2_DestroyComponent` _trunk_2)
                          (if (== (`self.Causer`) (`GameplayStatics.GetPlayerCharacter` 0))
                            (`/Game/Blueprints/BP_GameInstance.AchievementIncrease` (`self.InstanceRef`) (`|MakeArray` "NewEnumerator9" :!type "/Game/Blueprints/AchievementSystem/E_AchievementsTypes Enum"))))))))))))))))

(fn `UserConstructionScript`
  (`parent.UserConstructionScript`))
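; BP_FireballHazard is a fireball hazard actor that damages whatever overlaps its collider, applies status effects by damage type, then destroys itself.
; It caches the current level name on BeginPlay.
; In L_Tutorial2, overlapping the main character also moves that character's capsule to the TargetPoint location before damage is applied, using a hardcoded level-name check.
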(event `self.ReceiveBeginPlay`
  (bind _returnvalue (`GameplayStatics.GetCurrentLevelName` true))
  (set `self.levelName` _returnvalue))

(event `SetPlayerPosition`
  (`SceneComponent.K2_SetWorldLocation` (`Character.CapsuleComponent` (`self.playerRef`)) (`SceneComponent.K2_GetComponentLocation` (`/Game/Blueprints/EnemySpawner/BP_SpawnPoint.DefaultSceneRoot` (`self.targetPoint`))) false false))

(event `self.Collider.OnComponentBeginOverlap`
  (params (OverlappedComponent :type "PrimitiveComponent Object Reference") (OtherActor :type "Actor Object Reference") (OtherComp :type "PrimitiveComponent Object Reference") (OtherBodyIndex :type Integer) (bFromSweep :type Boolean) (SweepResult :type "HitResult Structure (by ref)"))
  (bind _asbp_main_character (cast `/Game/Blueprints/Character/Elizabeth/BP_MainCharacter` OtherActor)
    (:`then`
      (set `self.playerRef` _asbp_main_character)
      (if (`KismetStringLibrary.EqualEqual_StrStr` (`self.levelName`) "L_Tutorial2")
        (`self.SetPlayerPosition`)))
    (:`CastFailed`
      _))
  (`GameplayStatics.ApplyDamage` OtherActor (`self.Damage`) null self)
  (`/Game/Blueprints/Libraries/BP_Actor_FunctionLibrary.ApplyStatusEffects` OtherActor (`self.DamageType`) self)
  (`self.K2_DestroyActor`))

(fn `UserConstructionScript`)
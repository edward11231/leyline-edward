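; Spike trap hazard that springs when a pawn enters its trigger box, damaging actors in its damage box, until DisableTrap switches it off.
; After a short delay, a timeline raises the spikes and fires an Activate track that damages overlapping pawns and any later entrants, tracked to avoid repeat hits.
; A separate timeline retracts the spikes and re-arms the trap, avoiding re-firing the damage notify that reversing would cause.
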(event `self.Box.OnComponentBeginOverlap`
  (params (OverlappedComponent :type "PrimitiveComponent Object Reference") (OtherActor :type "Actor Object Reference") (OtherComp :type "PrimitiveComponent Object Reference") (OtherBodyIndex :type Integer) (bFromSweep :type Boolean) (SweepResult :type "HitResult Structure (by ref)"))
  (if (`self.Enabled`)
    (cast `Pawn` OtherActor)
    (if (`self.Triggerable`)
      (set `self.Triggerable` false)
      (`KismetArrayLibrary.Array_Clear` (`self.ActorsDamaged`))
      (`KismetSystemLibrary.Delay` 0.2)
      ;[1 1 1] Moves spikes and activates damage
      (bind (_direction _movespikes) (`Timeline|Timeline_0` :!via `PlayFromStart`)
        (:`Update`
          (bind _returnvalue_location (`KismetMathLibrary.BreakTransform` (`KismetMathLibrary.TLerp` (`SceneComponent.K2_GetComponentToWorld` (`self.StartingPoint`)) (`SceneComponent.K2_GetComponentToWorld` (`self.EndPoint`)) _movespikes)))
          (`SceneComponent.K2_SetWorldLocation` (`self.Spikes`) _returnvalue_location false false))
        (:`Finished`
          ;[1 1 1] Uses second timeline to reset trap instead of the reverse to not re-activate damage notify
          (`KismetSystemLibrary.Delay` 1.0)
          (set `self.active` false)
          (bind (_direction_2 _resettrack) (`Timeline|Timeline_1` :!via `PlayFromStart`)
            (:`Update`
              (bind _returnvalue_location_2 (`KismetMathLibrary.BreakTransform` (`KismetMathLibrary.TLerp` (`SceneComponent.K2_GetComponentToWorld` (`self.EndPoint`)) (`SceneComponent.K2_GetComponentToWorld` (`self.StartingPoint`)) _resettrack)))
              (`SceneComponent.K2_SetWorldLocation` (`self.Spikes`) _returnvalue_location_2 false false))
            (:`Finished`
              (set `self.Triggerable` true))))
        (:`Activate`
          (set `self.active` true)
          (`self.DamageAllOverlappingActors`))))))

(event `self.DamageBox.OnComponentBeginOverlap`
  (params (OverlappedComponent :type "PrimitiveComponent Object Reference") (OtherActor :type "Actor Object Reference") (OtherComp :type "PrimitiveComponent Object Reference") (OtherBodyIndex :type Integer) (bFromSweep :type Boolean) (SweepResult :type "HitResult Structure (by ref)"))
  ;[1 1 1] Deals damage during active frames
  (if (and (`self.active`) (not (`KismetArrayLibrary.Array_Contains` (`self.ActorsDamaged`) OtherActor)))
    (`KismetArrayLibrary.Array_Add` (`self.ActorsDamaged`) OtherActor)
    (`GameplayStatics.ApplyDamage` OtherActor (`self.damage`))))

(event `self.DisableTrap`
  (set `self.Enabled` false))

(fn `DamageAllOverlappingActors`
  (for _array_element (`PrimitiveComponent.GetOverlappingActors` (`self.DamageBox`) "/Script/Engine.Pawn")
    (`KismetArrayLibrary.Array_Add` (`self.ActorsDamaged`) _array_element)
    (`GameplayStatics.ApplyDamage` _array_element (`self.damage`))))

(fn `UserConstructionScript`
  (`parent.UserConstructionScript`))
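; Lava hazard actor that periodically applies fire status effects to actors inside its box volume.
; On BeginPlay it creates its own fire damage type object and fills its stats from the hazard's damage numbers.
; A looping timer then polls the box overlaps and applies that damage type to each actor, skipping those whose class is exactly BP_CandlekinKnight.
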(event `self.ReceiveBeginPlay`
  (bind (_damagenumbers_seconds _damagenumbers_damage _damagenumbers_iceslowpercentage _damagenumbers_windlaunchpower) (break `/Game/Blueprints/Attack/Struct_StatusEffectDamage` (`self.DamageNumbers`)))
  (bind _firetype (`/Game/Blueprints/Libraries/BP_Actor_FunctionLibrary.FireDamageType` self))
  (bind _output_get (set `self.DamageTypeRef` _firetype))
  (bind _asdamage_type_base (cast `/Game/Blueprints/DamageType_Base` _output_get))
  (setmembers `/Game/Blueprints/Attack/Struct_StatusEffectDamage` :`StructRef` (`/Game/Blueprints/DamageType_Base.Stats` _asdamage_type_base) :`Seconds` _damagenumbers_seconds :`Damage` _damagenumbers_damage :`IceSlowPercentage` _damagenumbers_iceslowpercentage :`WindLaunchPower` _damagenumbers_windlaunchpower)
  (`KismetSystemLibrary.K2_SetTimer` self "DamageAllActors" (`self.damageOverTime`) true))

(fn `DamageAllActors`
  (for _array_element (`PrimitiveComponent.GetOverlappingActors` (`self.Box`) "/Script/Engine.Actor")
    (if (not (== (`GameplayStatics.GetObjectClass` _array_element) "/Game/Blueprints/Character/Bosses/Candlekin/BP_CandlekinKnight.BP_CandlekinKnight_C"))
      (`/Game/Blueprints/Libraries/BP_Actor_FunctionLibrary.ApplyStatusEffects` _array_element (`self.DamageTypeRef`) self (`self.ignoreStack`)))))

(fn `UserConstructionScript`)
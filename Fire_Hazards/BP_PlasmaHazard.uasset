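; BP_PlasmaHazard is a timed area-of-effect hazard for Elizabeth's plasma cast, damaging enemies inside it.
; On BeginPlay it takes lifespan and horizontal scale from the player's ability stats, then computes damage over time from base DOT plus Plasma Refinement scaling.
; A looping one-second timer deals fire-typed damage to overlapping enemies, applies electric status effects, and feeds damage into the player's elemental burst progress.
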(event `self.ReceiveBeginPlay`
  (bind _plasmacastaoeradius (`/Game/Blueprints/Character/Elizabeth/PDA_PlayerAbilityStats.PlasmaCastAOERadius` (`/Game/Blueprints/Character/Elizabeth/BP_MainCharacter.ElizabethAbilityStats` (`self.PlayerRef`))))
  (bind _firetype (`/Game/Blueprints/Libraries/BP_Actor_FunctionLibrary.FireDamageType` self))
  (set `self.DamageType1` _firetype)
  (bind _electrictype (`/Game/Blueprints/Libraries/BP_Actor_FunctionLibrary.ElectricDamageType` self))
  (set `self.DamageType2` _electrictype)
  (`self.SetLifeSpan` (`/Game/Blueprints/Character/Elizabeth/PDA_PlayerAbilityStats.PlasmaCastAOEDuration` (`/Game/Blueprints/Character/Elizabeth/BP_MainCharacter.ElizabethAbilityStats` (`self.PlayerRef`))))
  (`SceneComponent.SetWorldScale3D` (`self.DefaultSceneRoot`) (`KismetMathLibrary.MakeVector` _plasmacastaoeradius _plasmacastaoeradius 0.05))
  (`KismetSystemLibrary.K2_SetTimer` self "ApplyStatusToAllActors" 1.0 true)
  (set `self.damageOverTime` (`self.GetDOTDamage`)))

(fn `ApplyStatusToAllActors`
  (for _array_element (`PrimitiveComponent.GetOverlappingActors` (`self.Box`) "/Game/Blueprints/Character/BP_BaseEnemy.BP_BaseEnemy_C")
    (bind _returnvalue (`GameplayStatics.ApplyDamage` _array_element (`self.damageOverTime`) null null (`GameplayStatics.GetObjectClass` (`self.DamageType1`))))
    (`/Game/Blueprints/Libraries/BP_Actor_FunctionLibrary.ApplyStatusEffects` _array_element (`self.DamageType2`) self (`self.ignoreStack`))
    (`/Game/Blueprints/Character/Elizabeth/BP_MainCharacter.UpdateElementalBurstProgress` (`self.PlayerRef`) _returnvalue)))

(fn `GetDOTDamage`
  (returns (ReturnValue :type "Float (double-precision)"))
  (bind _playerref (`self.PlayerRef`))
  (return (+ (* (`.PlasmaRefinement_22_63A3C5214945AFF0DBC4F2B1B8D55360` (break `/Game/Blueprints/Character/Struct_ElementUpgrades` (`.MagicElements_29_7A25D8F444438CC72BFFE9A360D5053C` (break `/Game/Blueprints/Character/Struct_PlayerStats` (`/Game/Blueprints/Character/Elizabeth/BP_MainCharacter.ElizabethStats` _playerref))))) (`/Game/Blueprints/Character/Elizabeth/PDA_PlayerAbilityStats.PlasmaCastRefinementDOTIncrease` (`/Game/Blueprints/Character/Elizabeth/BP_MainCharacter.ElizabethAbilityStats` _playerref))) (`/Game/Blueprints/Character/Elizabeth/PDA_PlayerAbilityStats.PlasmaCastDOT` (`/Game/Blueprints/Character/Elizabeth/BP_MainCharacter.ElizabethAbilityStats` _playerref)))))

(fn `UserConstructionScript`
  (`parent.UserConstructionScript`))
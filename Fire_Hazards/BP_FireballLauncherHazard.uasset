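; Fireball launcher trap that periodically shoots BP_FireballHazard projectiles from its spawn point.
; BeginPlay builds a fire damage type from the configured effect stats, then starts a looping Fire timer with an initial delay.
; Each shot passes damage, that shared damage type and RespawnPoint (as the fireball's TargetPoint) to the spawned actor.
; DisableTrap clears the timer, and ContinueFire restarts it.
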(event `ContinueFire`
  (`KismetSystemLibrary.K2_SetTimer` self "Fire" (`self.FireRate`) true (`self.InitialFireDelay`) :!label _label))

(event `self.ReceiveBeginPlay`
  (bind _firetype (`/Game/Blueprints/Libraries/BP_Actor_FunctionLibrary.FireDamageType` self))
  (bind _output_get (set `self.DamageType` _firetype))
  (`/Game/Blueprints/Libraries/BP_Actor_FunctionLibrary.SetEffectDamage` _output_get (`self.EffectStats`))
  (goto _label))

(event `self.DisableTrap`
  (`KismetSystemLibrary.K2_ClearTimer` self "Fire"))

(fn `Fire`
  (bind _spawnpoint (`self.SpawnPoint`))
  (`|SpawnActorFromClass` "/Game/Blueprints/Actors/Hazards/Fire_Hazards/BP_FireballHazard.BP_FireballHazard_C" (`KismetMathLibrary.MakeTransform` (`SceneComponent.K2_GetComponentLocation` _spawnpoint) (`SceneComponent.K2_GetComponentRotation` _spawnpoint)) "Undefined" "OverrideRootScale" null (`self.fireballDamage`) (`self.DamageType`) (`self.respawnPoint`) null))

(fn `UserConstructionScript`)
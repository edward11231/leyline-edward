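; Electric spinner hazard that rotates continuously and damages the player with two arrow-based line traces while active.
; A looping timer calls Activate to alternate active and cooldown states, toggling the particle effect.
; While active, Tick runs both traces behind a short Delay and applies damage when either hits the player.
; DisableTrap keeps it on cooldown from the next timer call; ToggleTempLasers is a disconnected stub.
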(event `self.ReceiveBeginPlay`
  (`self.ToggleTempLasers` false)
  (`KismetSystemLibrary.K2_SetTimer` self "Activate" (`self.cooldownTime`) true)
  (bind _asbp_main_character (cast `/Game/Blueprints/Character/Elizabeth/BP_MainCharacter` (`GameplayStatics.GetPlayerCharacter` 0)))
  (set `self.playerRef` _asbp_main_character))

(event `self.ReceiveTick`
  (params (DeltaSeconds :type "Float (single-precision)"))
  (bind (_start _end) (`self.ArrowTraceLocations` (`self.Arrow`)))
  (bind (_start_2 _end_2) (`self.ArrowTraceLocations` (`self.Arrow1`)))
  (`self.K2_AddActorLocalRotation` (`KismetMathLibrary.MakeRotator` 0.0 0.0 (* DeltaSeconds (`self.yawRotationSpeed`))))
  (if (not (`self.isOnCooldown`))
    (`KismetSystemLibrary.Delay` (`self.checkDelay`))
    (`|ExecutionSequence`
      (:`then_0`
        (bind (_outhit _returnvalue) (`KismetSystemLibrary.LineTraceSingleForObjects` :`Start` _start :`End` _end :`ObjectTypes` (`|MakeArray` "ObjectTypeQuery7" "ObjectTypeQuery1" :!type "EObjectTypeQuery Enum") :`DrawDebugType` (`self.debugSettings`)))
        (if (and _returnvalue (== (`.HitActor` (`GameplayStatics.BreakHitResult` _outhit)) (`self.playerRef`)))
          (`KismetSystemLibrary.PrintString` "Player hit")
          (`GameplayStatics.ApplyDamage` (`self.playerRef`) (`self.damage`) null self :!label _label)))
      (:`then_1`
        (bind (_outhit_2 _returnvalue_2) (`KismetSystemLibrary.LineTraceSingleForObjects` :`Start` _start_2 :`End` _end_2 :`ObjectTypes` (`|MakeArray` "ObjectTypeQuery7" "ObjectTypeQuery1" :!type "EObjectTypeQuery Enum") :`DrawDebugType` (`self.debugSettings`)))
        (if (and _returnvalue_2 (== (`.HitActor` (`GameplayStatics.BreakHitResult` _outhit_2)) (`self.playerRef`)))
          (`KismetSystemLibrary.PrintString` "Player hit")
          (goto _label))))))

(event `self.DisableTrap`
  (set `self.Enabled` false))

(fn `Activate`
  (if (`self.Enabled`)
    (if (`self.isOnCooldown`)
      (set `self.isOnCooldown` false)
      (`self.ToggleTempLasers` true)
      (`SceneComponent.SetVisibility` (`self.ParticleSystem`) true false)
      (else
        (set `self.isOnCooldown` true)
        (`self.ToggleTempLasers` false)
        (`SceneComponent.SetVisibility` (`self.ParticleSystem`) false false)))
    (else
      (set `self.isOnCooldown` true)
      (`SceneComponent.SetVisibility` (`self.ParticleSystem`) false false))))

(fn `ToggleTempLasers`
  (params (isLaserOn :type Boolean)))

(fn `UserConstructionScript`
  (`parent.UserConstructionScript`))
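; Electric hazard trap that cycles on and off and damages actors overlapping its box.
; A looping timer calls Activate, which despite its name toggles the active state and both particle systems.
; While active and enabled, Tick uses a Delay to pace damage to every overlapping actor.
; DisableTrap shuts it off by clearing Enabled, hiding the particles and stopping the timer.
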(event `self.ReceiveBeginPlay`
  (`parent.ReceiveBeginPlay`)
  (`/Game/Blueprints/Libraries/BP_Actor_FunctionLibrary.ElectricDamageType` self)
  (`KismetSystemLibrary.K2_SetTimer` self "Activate" (`self.trapCycleOnTime`) true))

(event `self.ReceiveTick`
  (params (DeltaSeconds :type "Float (single-precision)"))
  (if (and (`self.isTrapActive`) (`self.Enabled`))
    (`KismetSystemLibrary.Delay` (`self.damageDelay`))
    (for _array_element (`PrimitiveComponent.GetOverlappingActors` (`self.Box`) "/Script/Engine.Actor")
      (`GameplayStatics.ApplyDamage` _array_element (`self.damage`) null self))))

(event `self.DisableTrap`
  (set `self.Enabled` false)
  (`SceneComponent.SetVisibility` (`self.ParticleSystem`) false false)
  (`SceneComponent.SetVisibility` (`self.ParticleSystem1`) false false)
  (`KismetSystemLibrary.K2_ClearTimer` self "Activate"))

(fn `Activate`
  (if (`self.isTrapActive`)
    (`KismetSystemLibrary.PrintString` "Trap is off")
    (set `self.isTrapActive` false)
    (`SceneComponent.SetVisibility` (`self.ParticleSystem`) false false)
    (`SceneComponent.SetVisibility` (`self.ParticleSystem1`) false false)
    (else
      (`KismetSystemLibrary.PrintString` "Trap is on")
      (set `self.isTrapActive` true)
      (`SceneComponent.SetVisibility` (`self.ParticleSystem`) true false)
      (`SceneComponent.SetVisibility` (`self.ParticleSystem1`) true false))))

(fn `Deactivate`
  (`KismetSystemLibrary.PrintString` "Trap is off")
  (if (`self.isTrapActive`)
    (set `self.isTrapActive` false)))

(fn `UserConstructionScript`
  (`parent.UserConstructionScript`))
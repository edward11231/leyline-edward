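; Lightning rod trap hazard that electrocutes actors around it when the main character comes near.
; Box overlaps track player presence, and Tick fires a DoOnce-gated cycle while the trap is enabled.
; Each cycle attaches a lightning effect, waits the activation time, damages every actor in HitRadius, then resets to repeat.
; DisableTrap stops new cycles, but a strike already charging still lands.
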(event `Reset`
  (goto _label :!via `Reset`))

(event `self.ReceiveTick`
  (params (DeltaSeconds :type "Float (single-precision)"))
  (if (and (`self.Enabled`) (`self.inRadius`))
    (`/Engine/EditorBlueprintResources/StandardMacros.DoOnce` false :!label _label
      (:`Completed`
        (`GameplayStatics.SpawnEmitterAttached` "/Game/VFX/Automaton/PS_LightingTrap.PS_LightingTrap" (`self.ChildActor`))
        (`KismetSystemLibrary.Delay` (`self.activationTime`))
        (`self.Electrocute`)
        (`self.Reset`)))))

(event `self.ReceiveBeginPlay`
  (`/Game/Blueprints/Libraries/BP_Actor_FunctionLibrary.ElectricDamageType` self))

(event `self.Box.OnComponentBeginOverlap`
  (params (OverlappedComponent :type "PrimitiveComponent Object Reference") (OtherActor :type "Actor Object Reference") (OtherComp :type "PrimitiveComponent Object Reference") (OtherBodyIndex :type Integer) (bFromSweep :type Boolean) (SweepResult :type "HitResult Structure (by ref)"))
  (cast `/Game/Blueprints/Character/Elizabeth/BP_MainCharacter` OtherActor)
  (set `self.inRadius` true))

(event `self.Box.OnComponentEndOverlap`
  (params (OverlappedComponent :type "PrimitiveComponent Object Reference") (OtherActor :type "Actor Object Reference") (OtherComp :type "PrimitiveComponent Object Reference") (OtherBodyIndex :type Integer))
  (cast `/Game/Blueprints/Character/Elizabeth/BP_MainCharacter` OtherActor)
  (set `self.inRadius` false))

(event `self.DisableTrap`
  (set `self.Enabled` false))

(fn `Electrocute`
  (for _array_element (`PrimitiveComponent.GetOverlappingActors` (`self.HitRadius`) "/Script/Engine.Actor")
    (`GameplayStatics.ApplyDamage` _array_element (`self.damage`) null self)
    (`KismetSystemLibrary.PrintString` "ZAPPING!")))

(fn `UserConstructionScript`
  (`parent.UserConstructionScript`))
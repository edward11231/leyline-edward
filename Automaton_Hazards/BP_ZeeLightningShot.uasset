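; BP_ZeeLightningShot is a one-shot lightning hazard that strikes actors inside its sphere after a configurable delay.
; BeginPlay sets a timer for HitTarget, which attaches the lightning particle effect and passes each overlapping actor to Hit.
; Hit applies HazardDamage after a short Delay, which is shared across the loop's calls, so only one actor takes damage.
; The hazard then destroys itself after a further pause.
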(event `self.ReceiveBeginPlay`
  (`KismetSystemLibrary.K2_SetTimer` self "HitTarget" (`self.delay`)))

(event `DestroyActor`
  (`KismetSystemLibrary.Delay` 2.0)
  (`self.K2_DestroyActor`))

(event `Hit`
  (params (DamagedActor :type "Actor Object Reference"))
  (`KismetSystemLibrary.Delay` 1.0)
  (`GameplayStatics.ApplyDamage` DamagedActor (`self.hazardDamage`)))

(fn `HitTarget`
  (`GameplayStatics.SpawnEmitterAttached` "/Game/VFX/Automaton/PS_LightingTrap.PS_LightingTrap" (`self.ChildActor`))
  (for _array_element (`PrimitiveComponent.GetOverlappingActors` (`self.Sphere`) "/Script/Engine.Actor")
    (`self.Hit` _array_element))
  (`self.DestroyActor`))

(fn `UserConstructionScript`)